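; A test actor that starts a dialogue by its Key through the DialogueSubsystem on BeginPlay.
; An unconnected animation test finds the player battle character and branches on its current weapon type.
; That dormant branch steps the weapon from None through Sword and Spear to Fist, playing an animation by AnimKey, and at Fist plays a Sword montage instead.
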(event EventBeginPlay
  (Class|DialogueSubsystem|StartDialoguebyKey (Subsystems|GetDialogueSubsystem) (Variables|Default|GetKey)))

(fn ConstructionScript)