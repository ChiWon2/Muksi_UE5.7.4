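; Test quest objective actor that reports progress to its objective component when its collision box is overlapped.
; On BeginPlay it adds two test quests from the ForTest table through the quest subsystem and binds the box's begin overlap to NotifyObjective, with no filter on the overlapping actor.
; It also hooks the Muksi player controller's P input to debug-print the modal widget stack.
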(event Custom|OnComponentBeginOverlap_Event
  (params (OverlappedComponent :type Primitive%20Component%20Object%20Reference) (OtherActor :type Actor%20Object%20Reference) (OtherComp :type Primitive%20Component%20Object%20Reference) (OtherBodyIndex :type Integer) (bFromSweep :type Boolean) (SweepResult :type Hit%20Result%20Structure%20%28by%20ref%29))
  (Class|ObjectiveActorComponent|NotifyObjective (Variables|Default|GetObjectiveActor) 1))

(event Custom|CustomEvent
  (Class|MuksiUISubsystem|DebugPrintWidgetStack (Subsystems|GetMuksiUISubsystem) (GameplayTags|MakeLiteralGameplayTag "(TagName=\"Muksi.WidgetStack.Modal\")")))

(event EventBeginPlay
  (bind _returnvalue (Subsystems|GetQuestSubsystem))
  (EventDispatchers|BindEventtoOnPPressedInput (Class|MuksiFunctionLibrary|GetMuksiPlayerController) (delegate Custom|CustomEvent))
  (Class|QuestSubsystem|AddNewQuest _returnvalue (Utilities|Struct|MakeQuestKey "ForTest" "TestTest"))
  (Collision|AssignOnComponentBeginOverlap (Variables|Default|GetBox) (delegate Custom|OnComponentBeginOverlap_Event))
  (Class|QuestSubsystem|AddNewQuest _returnvalue (Utilities|Struct|MakeQuestKey "ForTest" "TestInventory")))

(fn ConstructionScript)